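; BP_CAPlayerState is the player state for the carpenter game, tracking the product a player is carrying.
; OnPickup stores the held product and sets a holding flag.
; OnDeliver passes the product's data to the game state's DeliverOrder, then clears the flag and destroys the product actor.
; Both events run from server calls in other classes, so they are not replicated.
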(event `OnPickup`
  (params (Product :type "/Game/CarpenterGame/Blueprints/IntractableActors/BP_Product Object Reference"))
  ; Pickup and Deliver Product. Both are called from Server events form other classes, so they don't need to be replicated.
  (set `self.CurrentlyHeldProduct` Product)
  (set `self.bIsHoldingProduct` true))

(event `OnDeliver`
  (bind _cagamestate (`self.GetCAGameState`))
  ; Pickup and Deliver Product. Both are called from Server events form other classes, so they don't need to be replicated.
  (`/Engine/EditorBlueprintResources/StandardMacros.IsValid` _cagamestate
    (:`Is Valid`
      (`/Game/CarpenterGame/Blueprints/BP_CAGameStateBase.DeliverOrder` _cagamestate (`/Game/CarpenterGame/Blueprints/IntractableActors/BP_Product.ProductData` (`self.CurrentlyHeldProduct`)))
      (set `self.bIsHoldingProduct` false)
      (`self.K2_DestroyActor` (`self.CurrentlyHeldProduct`))
      (set `self.CurrentlyHeldProduct` null))))

(fn `GetCAGameState`
  (returns (CAGameState :type "/Game/CarpenterGame/Blueprints/BP_CAGameStateBase Object Reference"))
  (return (cast `/Game/CarpenterGame/Blueprints/BP_CAGameStateBase` (`GameplayStatics.GetGameState`) :!pure true)))

(fn `UserConstructionScript`)