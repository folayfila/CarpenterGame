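; Game state for the carpenter game that runs the product order queue, shared budget and available product spots.
; The server adds random type-and-color orders on a random repeating timer, up to a cap.
; Deliveries remove the best-matching order and pay full for exact matches or half for type-only.
; Budget and Orders RepNotifies refresh the local player's HUD, alongside helpers for enum text, colors and spot lookup.
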(event `self.ReceiveBeginPlay`
  ; BeginPlay: Generating a new order every couple of seconds (random value from Min-Max).
  ;;[0.15 0.01641 0.01641 0.5 15] Only the server can should set the timer!
  (`/Engine/EditorBlueprintResources/ActorMacros.Switch Has Authority`
    (:`Authority`
      (`KismetSystemLibrary.K2_SetTimerDelegate` (delegate `RequestOrder`) (`KismetMathLibrary.RandomFloatInRange` (`self.MinOrderInterval`) (`self.MaxOrderInterval`)))
      ;;[0.15 0.15 0.15 0.5 15] Add Max number of slots and set them to be available
      (for _ (range (`self.MaxNumberOfProductsAtOnce`))
        (`KismetArrayLibrary.Array_Add` (`self.AvailableProductSpots`) true)))))

(event `RequestOrder`
  ; BeginPlay: Generating a new order every couple of seconds (random value from Min-Max).
  (if (< (`KismetArrayLibrary.Array_Length` (`self.Orders`)) (`self.MaxNumberOfOrders`))
    (`KismetArrayLibrary.Array_Add` (`self.Orders`) (`self.GenerateRandomOrder`))
    (`self.UpdatePlayerUI`))
  ;;[0.15 0.15 0.15 0.5 15] Start a new timer
  (`KismetSystemLibrary.K2_SetTimerDelegate` (delegate `RequestOrder`) (`KismetMathLibrary.RandomFloatInRange` (`self.MinOrderInterval`) (`self.MaxOrderInterval`))))

(event `DeliverOrder`
  (params (Order :type "/Game/CarpenterGame/Misc/FOrder Structure"))
  ; Deliver Order: Updates the orders list and budget based on the delivery.
  (bind _result (`self.DeliverOrderAndGetResults` Order))
  (set `self.Budget` (+ (`self.Budget`) (`self.GetAddedBudgetFromScore` _result)))
  (`self.UpdatePlayerUI`))

(fn `CanSpawnProduct`
  (returns (bAllowed :type Boolean))
  ; Return true if at least one spot is available
  (return (!= (`KismetArrayLibrary.Array_Find` (`self.AvailableProductSpots`) true) -1)))

(fn `DeliverOrderAndGetResults`
  (params (Order :type "/Game/CarpenterGame/Misc/FOrder Structure"))
  (returns (Result :type Integer))
  (locals (Score :type Integer :default 0) (BestOrderIndex :type Integer :default -1))
  (bind (_type _color) (break `/Game/CarpenterGame/Misc/FOrder` Order))
  ;[0.15 0.15 0.15 0] Compares the passed order with the list of orders. Returns an int Score, 2 for a perfect match, 1 for a type only match, 0 for no match.
  (for (_array_element _array_index) (`self.Orders`)
    (bind (_type_2 _color_2) (break `/Game/CarpenterGame/Misc/FOrder` _array_element))
    (bind _returnvalue (`|EnumEquality` _type _type_2))
    ;;[0.15 0.15 0.15 0.5 15] Compare the types first. If the types don't match, skip.
    (if _returnvalue
      ;;[0.06934 0.15 0.08027 0.5 15] Color check, if perfect match. Max score, break immediatly
      (if (and _returnvalue (`|EnumEquality` _color _color_2))
        (set `local.BestOrderIndex` _array_index)
        (set `local.Score` 2)
        (break)
        (else
          ;;[0.15 0.1248 0.06969 0.5 15] If only the type matches, update the best index only if it wasn't already set. Otherwise ignore as we pick the first match.
          (if (== (`local.BestOrderIndex`) -1)
            (set `local.BestOrderIndex` _array_index)
            (set `local.Score` 1))))))
  ;;[0.15 0.15 0.15 0.5 15] If the best index is greater than -1 (default), then we found a match. Remove it from the list of orders.
  (if (> (`local.BestOrderIndex`) -1)
    (`KismetArrayLibrary.Array_Remove` (`self.Orders`) (`local.BestOrderIndex`)))
  (return (`local.Score`)))

(fn `FindFirstAvailableSpot`
  (returns (AvailableSpot :type Integer))
  (return (`KismetArrayLibrary.Array_Find` (`self.AvailableProductSpots`) true)))

(fn `GenerateRandomOrder`
  (returns (NewOrder :type "/Game/CarpenterGame/Misc/FOrder Structure"))
  ; Generating a random FOrder by using random integer in range from 0 to the last enum value in each order enum.
  (return (make `/Game/CarpenterGame/Misc/FOrder` (cast `/Game/CarpenterGame/Misc/EProductTypes` (`KismetMathLibrary.Conv_IntToByte` (`KismetMathLibrary.RandomIntegerInRange` 1 (- (enumcount `/Game/CarpenterGame/Misc/EProductTypes`) 1)))) (cast `/Game/CarpenterGame/Misc/EColors` (`KismetMathLibrary.Conv_IntToByte` (`KismetMathLibrary.RandomIntegerInRange` 0 (- (enumcount `/Game/CarpenterGame/Misc/EColors`) 1)))))))

(fn `GetAddedBudgetFromScore`
  (params (Score :type Integer))
  (returns (AddedBudget :type "Float (double-precision)"))
  (locals (Amount :type "Float (double-precision)" :default 0.0))
  ; Switch on score. 2 = Full Amount | 1 = Half Amount | Anything else = 0
  (switch `int` Score
    (:`Default`
      (set `local.Amount` 0.0))
    (:`0`
      (set `local.Amount` 0.0))
    (:`1`
      (set `local.Amount` (/ (`self.PaymentPerCorrectOrder`) 2.0)))
    (:`2`
      (set `local.Amount` (`self.PaymentPerCorrectOrder`))))
  (return (`local.Amount`)))

(fn `GetColorAsText`
  (params (Color :type "/Game/CarpenterGame/Misc/EColors Enum" :default "NewEnumerator0"))
  (returns (ColorText :type Text))
  (locals (Result :type Text))
  ; Helper that returns the EColors type as Text. Update if new types are added!
  (switch `/Game/CarpenterGame/Misc/EColors` Color
    (:`NewEnumerator0`
      (set `local.Result` "Brown"))
    (:`NewEnumerator1`
      (set `local.Result` "Red"))
    (:`NewEnumerator2`
      (set `local.Result` "Green"))
    (:`NewEnumerator3`
      (set `local.Result` "Blue"))
    (:`NewEnumerator4`
      (set `local.Result` "Purple"))
    (:`NewEnumerator5`
      (set `local.Result` "Black"))
    (:`NewEnumerator6`
      (set `local.Result` "White")))
  (return (`local.Result`)))

(fn `GetLinearColor`
  (params (ColorType :type "/Game/CarpenterGame/Misc/EColors Enum" :default "NewEnumerator0"))
  (returns (Color :type "LinearColor Structure"))
  (locals (NewColor :type "LinearColor Structure"))
  ; Helper that returns a Linera Color based on EColors type. Update if new EColors are added!
  (switch `/Game/CarpenterGame/Misc/EColors` ColorType
    (:`NewEnumerator0`
      (set `local.NewColor` (struct :`R` 0.109375 :`G` 0.01356 :`B` 0.013508 :`A` 1.0)))
    (:`NewEnumerator1`
      (set `local.NewColor` (struct :`R` 0.973958 :`G` 0.000528 :`A` 1.0)))
    (:`NewEnumerator2`
      (set `local.NewColor` (struct :`G` 0.880208 :`B` 0.053447 :`A` 1.0)))
    (:`NewEnumerator3`
      (set `local.NewColor` (struct :`G` 0.112593 :`B` 0.880208 :`A` 1.0)))
    (:`NewEnumerator4`
      (set `local.NewColor` (struct :`R` 0.396836 :`B` 0.75 :`A` 1.0)))
    (:`NewEnumerator5`
      (set `local.NewColor` (struct :`A` 1.0)))
    (:`NewEnumerator6`
      (set `local.NewColor` (struct :`R` 1.0 :`G` 1.0 :`B` 1.0 :`A` 1.0))))
  (return (`local.NewColor`)))

(fn `GetProductTypeAsText`
  (params (Type :type "/Game/CarpenterGame/Misc/EProductTypes Enum" :default "NewEnumerator0"))
  (returns (TypeText :type Text))
  (locals (Result :type Text))
  ;[0.1304 0.09789 0.15 0.5] Helper that gets the product type as Text. Update if new types are added!
  (switch `/Game/CarpenterGame/Misc/EProductTypes` Type
    (:`NewEnumerator0`
      (set `local.Result` ""))
    (:`NewEnumerator1`
      (set `local.Result` "Plank"))
    (:`NewEnumerator2`
      (set `local.Result` "Chair"))
    (:`NewEnumerator3`
      (set `local.Result` "Table"))
    (:`NewEnumerator4`
      (set `local.Result` "Shelf")))
  (return (`local.Result`)))

(fn `OnRep_Budget`
  (`self.UpdatePlayerUI`))

(fn `OnRep_Orders`
  (`self.UpdatePlayerUI`))

(fn `UpdatePlayerUI`
  ; Call a client only "UpdateUI" on the local player controller. Break once found.
  (for _array_element (`self.PlayerArray`)
    (bind _asbp_caplayer_controller (cast `/Game/CarpenterGame/Blueprints/BP_CAPlayerController` (`PlayerState.GetPlayerController` _array_element)))
    (if (`Controller.IsLocalPlayerController` _asbp_caplayer_controller)
      (`/Game/CarpenterGame/Blueprints/BP_CAPlayerController.Client_UpdatHUD` _asbp_caplayer_controller)
      (break))))

(fn `UserConstructionScript`)