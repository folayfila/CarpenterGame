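; BP_Product is an interactable, paintable product that players pick up and carry.
; Interaction goes through a server event that checks the player's product state, attaches the product to the character's hold point, notifies the player state and frees its spawn spot in the game state.
; A per-instance dynamic material created at BeginPlay lets the color update event change the mesh color alongside the product's order data.
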(event `self.ReceiveBeginPlay`
  ;[0.0985 0.15 0.1117 0.5] Create a dynamic material instance per product so we can change the color param in real time when the product is painted.
  (bind _returnvalue (`PrimitiveComponent.CreateDynamicMaterialInstance` (`self.Mesh`) 0 "/Game/CarpenterGame/Materials/M_ColorBase.M_ColorBase" "None"))
  (set `self.MeshMaterial` _returnvalue))

(event `/Game/CarpenterGame/Blueprints/IntractableActors/BPI_Interactable.Interact`
  (params (InteractingCharacter :type "/Game/CarpenterGame/Blueprints/BP_CACharacter Object Reference"))
  ; Interact Implemetation
  (`self.Server_OnInteract` InteractingCharacter))

(event `Server_OnInteract`
  (params (`Interacting Character` :type "/Game/CarpenterGame/Blueprints/BP_CACharacter Object Reference"))
  (bind _caplayerstate (`/Game/CarpenterGame/Blueprints/BP_CACharacter.GetCAPlayerState` `Interacting Character`))
  ; Interact Implemetation
  (if (`|EnumEquality` (`/Game/CarpenterGame/Blueprints/BP_CAPlayerState.ProductState` _caplayerstate) "NewEnumerator0")
    (`self.K2_AttachToComponent` (`/Game/CarpenterGame/Blueprints/BP_CACharacter.HoldPoint` `Interacting Character`) "None" "SnapToTarget" "SnapToTarget" "KeepWorld")
    (`/Game/CarpenterGame/Blueprints/BP_CAPlayerState.OnPickup` _caplayerstate self)
    (if (!= (`self.SpawnSpotIndex`) -1)
      (`KismetArrayLibrary.Array_Set` (`/Game/CarpenterGame/Blueprints/BP_CAGameStateBase.AvailableProductSpots` (`self.GetCAGameState`)) (`self.SpawnSpotIndex`) true)
      (set `self.SpawnSpotIndex` -1))))

(event `Server_UpdateProductColor`
  (params (Color :type "/Game/CarpenterGame/Misc/EColors Enum" :default "NewEnumerator0"))
  (bind _productdata_type (break `/Game/CarpenterGame/Misc/FOrder` (`self.ProductData`)))
  ; Update the color data and the mesh's color on server and all clients
  (bind _output_get (set `self.ProductData` (make `/Game/CarpenterGame/Misc/FOrder` _productdata_type Color)))
  (`MaterialInstanceDynamic.SetVectorParameterValue` (`self.MeshMaterial`) "Color" (`/Game/CarpenterGame/Blueprints/BP_CAGameStateBase.GetLinearColor` (`self.GetCAGameState`) (`.Color_7_BB3B9ED848117EF2D49BCEA45E3891B1` (break `/Game/CarpenterGame/Misc/FOrder` _output_get)))))

(fn `UserConstructionScript`
  (`parent.UserConstructionScript`))