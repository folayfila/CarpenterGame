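; BP_PaintCan is an interactable paint can that applies its color type to the product a player is painting.
; On BeginPlay it creates a dynamic material from M_ColorBase and tints its mesh with the color the game state returns for its ColorType.
; On Interact it checks that the player state's product state is painting, then calls ServerUpdateProductColor on the held product.
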(event `self.ReceiveBeginPlay`
  ;[0.0985 0.15 0.1117 0.5] Create a dynamic material instance per paint can and set it to the passed color on spawn.
  (bind _returnvalue (`PrimitiveComponent.CreateDynamicMaterialInstance` (`self.Mesh`) 0 "/Game/CarpenterGame/Materials/M_ColorBase.M_ColorBase" "None"))
  (`MaterialInstanceDynamic.SetVectorParameterValue` _returnvalue "Color" (`/Game/CarpenterGame/Blueprints/BP_CAGameStateBase.GetLinearColor` (`self.GetCAGameState`) (`self.Color Type`))))

(event `/Game/CarpenterGame/Blueprints/IntractableActors/BPI_Interactable.Interact`
  (params (InteractingCharacter :type "/Game/CarpenterGame/Blueprints/BP_CACharacter Object Reference"))
  ; Interact implementation: Update the player's held product color ONLY if they're painting it.
  (bind _asbp_caplayer_state (cast `/Game/CarpenterGame/Blueprints/BP_CAPlayerState` (`Pawn.PlayerState` InteractingCharacter)))
  (if (`|EnumEquality` (`/Game/CarpenterGame/Blueprints/BP_CAPlayerState.PlayerProductState` _asbp_caplayer_state) "NewEnumerator2")
    (`/Game/CarpenterGame/Blueprints/IntractableActors/BP_Product.Server_UpdateProductColor` (`/Game/CarpenterGame/Blueprints/BP_CAPlayerState.CurrentlyHeldProduct` _asbp_caplayer_state) (`self.Color Type`))))

(fn `UserConstructionScript`
  (`parent.UserConstructionScript`))