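; BP_ProductionMachine is an interactable machine that spawns the product type a player has selected.
; On Interact, it checks that the game state allows spawning and the player state holds a non-default selection, then calls a server spawn event.
; That event spawns a BP_Product with default color, offset along world X by the game state's spawned count, then resets the selection and increments the count.
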(event `/Game/CarpenterGame/Blueprints/IntractableActors/BPI_Interactable.Interact`
  (params (InteractingCharacter :type "/Game/CarpenterGame/Blueprints/BP_CACharacter Object Reference"))
  (bind _asbp_caplayer_state (cast `/Game/CarpenterGame/Blueprints/BP_CAPlayerState` (`Pawn.PlayerState` InteractingCharacter)))
  (if (and (`/Game/CarpenterGame/Blueprints/BP_CAGameStateBase.CanSpawnProduct` (`self.GetCAGameState`)) (`|EnumInequality` (`/Game/CarpenterGame/Blueprints/BP_CAPlayerState.SelectedProductType` _asbp_caplayer_state) "NewEnumerator0"))
    (`self.Server_SpawnProduct` _asbp_caplayer_state)))

(event `Server_SpawnProduct`
  (params (PlayerState :type "/Game/CarpenterGame/Blueprints/BP_CAPlayerState Object Reference"))
  (bind _cagamestatebase (`self.GetCAGameState`))
  (bind (_returnvalue_x _returnvalue_y _returnvalue_z) (`KismetMathLibrary.BreakVector` (`SceneComponent.K2_GetComponentLocation` (`self.SpawnLocation`))))
  (`|SpawnActorFromClass` "/Game/CarpenterGame/Blueprints/IntractableActors/BP_Product.BP_Product_C" (`KismetMathLibrary.MakeTransform` (`KismetMathLibrary.MakeVector` (+ _returnvalue_x (* (`/Game/CarpenterGame/Blueprints/BP_CAGameStateBase.CurrentSpawnedProductsNum` (`self.GetCAGameState`)) 100)) _returnvalue_y _returnvalue_z) (`self.K2_GetActorRotation`)) "Undefined" "MultiplyWithRoot" null (make `/Game/CarpenterGame/Misc/FOrder` (`/Game/CarpenterGame/Blueprints/BP_CAPlayerState.SelectedProductType` PlayerState)) null)
  (set `/Game/CarpenterGame/Blueprints/BP_CAPlayerState.SelectedProductType` "NewEnumerator0" PlayerState)
  (set `/Game/CarpenterGame/Blueprints/BP_CAGameStateBase.CurrentSpawnedProductsNum` (+ (`/Game/CarpenterGame/Blueprints/BP_CAGameStateBase.CurrentSpawnedProductsNum` _cagamestatebase) 1) _cagamestatebase))

(fn `UserConstructionScript`
  (`parent.UserConstructionScript`))