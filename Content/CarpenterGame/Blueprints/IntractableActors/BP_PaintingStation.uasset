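; Interactable painting station that holds a player's product and exposes one paint can per color while a product is on it.
; On BeginPlay it spawns a BP_PaintCan for each EColors value, spaced along world X from SprayCanStartLocation.
; Interact attaches the player's held product to the station mesh, or returns the stored one to the player's HoldPoint.
; Cans are toggled through their Visibility and Camera collision responses, staying ignored while the station is empty.
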(event `self.ReceiveBeginPlay`
  (bind (_returnvalue_x _returnvalue_y _returnvalue_z) (`KismetMathLibrary.BreakVector` (`SceneComponent.K2_GetComponentLocation` (`self.SprayCanStartLocation`))))
  ; Spawn cans with an offset based on the number of existing colors in EColors.
  (bind _enumvalue (foreach `/Game/CarpenterGame/Misc/EColors` true)
    (:`LoopBody`
      (bind _returnvalue (`|SpawnActorFromClass` "/Game/CarpenterGame/Blueprints/IntractableActors/BP_PaintCan.BP_PaintCan_C" (`KismetMathLibrary.MakeTransform` (`KismetMathLibrary.MakeVector` (+ _returnvalue_x (* (`KismetMathLibrary.Conv_ByteToInt` _enumvalue) 100)) _returnvalue_y _returnvalue_z) (`self.K2_GetActorRotation`)) "Undefined" "MultiplyWithRoot" null _enumvalue null))
      (`KismetArrayLibrary.Array_Add` (`self.PaintCans`) _returnvalue))
    (:`then`
      (`self.SetPaintCansEnabled` false))))

(event `/Game/CarpenterGame/Blueprints/IntractableActors/BPI_Interactable.Interact`
  (params (InteractingCharacter :type "/Game/CarpenterGame/Blueprints/BP_CACharacter Object Reference"))
  (bind _asbp_caplayer_state (cast `/Game/CarpenterGame/Blueprints/BP_CAPlayerState` (`Pawn.PlayerState` InteractingCharacter)))
  (`/Engine/EditorBlueprintResources/StandardMacros.IsValid` (`self.Product`)
    (:`Is Valid`
      (`self.K2_AttachToComponent` (`self.Product`) (`/Game/CarpenterGame/Blueprints/BP_CACharacter.HoldPoint` InteractingCharacter) "None" "SnapToTarget" "SnapToTarget" "KeepWorld" true)
      (set `self.Product` null)
      (`self.SetPaintCansEnabled` false))
    (:`Is Not Valid`
      (bind _currentlyheldproduct (`/Game/CarpenterGame/Blueprints/BP_CAPlayerState.CurrentlyHeldProduct` _asbp_caplayer_state))
      (`self.K2_AttachToComponent` _currentlyheldproduct (`self.Mesh`) "None" "SnapToTarget" "SnapToTarget" "KeepWorld" true)
      (set `self.Product` _currentlyheldproduct)
      (`self.SetPaintCansEnabled` true))))

(fn `SetPaintCansEnabled`
  (params (bEnabled :type Boolean))
  (for _array_element (`self.PaintCans`)
    (if bEnabled
      (bind _mesh (`/Game/CarpenterGame/Blueprints/IntractableActors/BP_InteractableActorBase.Mesh` _array_element))
      (`PrimitiveComponent.SetCollisionResponseToChannel` _mesh "ECC_Visibility" "ECR_Block")
      (`PrimitiveComponent.SetCollisionResponseToChannel` _mesh "ECC_Camera" "ECR_Block")
      (else
        (bind _mesh_2 (`/Game/CarpenterGame/Blueprints/IntractableActors/BP_InteractableActorBase.Mesh` _array_element))
        (`PrimitiveComponent.SetCollisionResponseToChannel` _mesh_2 "ECC_Visibility" "ECR_Ignore")
        (`PrimitiveComponent.SetCollisionResponseToChannel` _mesh_2 "ECC_Camera" "ECR_Ignore")))))

(fn `UserConstructionScript`
  (`parent.UserConstructionScript`))