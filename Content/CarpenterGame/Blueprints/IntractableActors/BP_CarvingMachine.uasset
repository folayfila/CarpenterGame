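; BP_CarvingMachine is an interactable machine that spawns the product type selected in the interacting player's state.
; Interact checks that the game state can spawn a product and the player's selection is not the default, then calls the server spawn event.
; That event spawns a BP_Product with default color at the first available spot along SpawnLocation's forward axis, resets the selection, and updates the game state's spot array.
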(event `/Game/CarpenterGame/Blueprints/IntractableActors/BPI_Interactable.Interact`
  (params (InteractingCharacter :type "/Game/CarpenterGame/Blueprints/BP_CACharacter Object Reference"))
  (bind _asbp_caplayer_state (cast `/Game/CarpenterGame/Blueprints/BP_CAPlayerState` (`Pawn.PlayerState` InteractingCharacter)))
  (if (and (`/Game/CarpenterGame/Blueprints/BP_CAGameStateBase.CanSpawnProduct` (`self.GetCAGameState`)) (`|EnumInequality` (`/Game/CarpenterGame/Blueprints/BP_CAPlayerState.SelectedProductType` _asbp_caplayer_state) "NewEnumerator0"))
    (`self.Server_SpawnProduct` _asbp_caplayer_state)))

(event `Server_SpawnProduct`
  (params (PlayerState :type "/Game/CarpenterGame/Blueprints/BP_CAPlayerState Object Reference"))
  (bind _spawnlocation (`self.SpawnLocation`))
  (bind _availablespot (`/Game/CarpenterGame/Blueprints/BP_CAGameStateBase.FindFirstAvailableSpot` (`self.GetCAGameState`)))
  (`|SpawnActorFromClass` "/Game/CarpenterGame/Blueprints/IntractableActors/BP_Product.BP_Product_C" (`KismetMathLibrary.MakeTransform` (+ (`SceneComponent.K2_GetComponentLocation` _spawnlocation) (* (`SceneComponent.GetForwardVector` _spawnlocation) (* _availablespot 100))) (`self.K2_GetActorRotation`)) "Undefined" "MultiplyWithRoot" null (make `/Game/CarpenterGame/Misc/FOrder` (`/Game/CarpenterGame/Blueprints/BP_CAPlayerState.SelectedProductType` PlayerState)) _availablespot null)
  (set `/Game/CarpenterGame/Blueprints/BP_CAPlayerState.SelectedProductType` "NewEnumerator0" PlayerState)
  (`KismetArrayLibrary.Array_Set` (`/Game/CarpenterGame/Blueprints/BP_CAGameStateBase.AvailableProductSpots` (`self.GetCAGameState`)) _availablespot))

(fn `UserConstructionScript`
  (`parent.UserConstructionScript`))